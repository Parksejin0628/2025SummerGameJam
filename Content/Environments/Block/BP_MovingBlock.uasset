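; BP_MovingBlock is a block actor that oscillates from its starting position along MovementDir, up to 300 units times that vector.
; Tick accumulates time scaled by AlphaScale and folds it into a triangle wave with modulo and Abs to drive the Lerp offset.
; Its MergeBlock override works in stages: one block type shows the widget and arms IsTime.
; A second type then hides the widget, sets AlphaScale and destroys the collision component.
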(event EventBeginPlay
  (|CallParentFunction)
  (Variables|Default|SetDefaultLocation (Transformation|GetActorLocation)))

(event Collision|EventActorBeginOverlap
  (params (OtherActor :type Actor%20Object%20Reference))
  (|CallParentFunction OtherActor) ; This node is disabled and will not be called.\nDrag off pins to build functionality.
)

(event EventTick
  (params (DeltaSeconds :type Float%20%28single-precision%29))
  (bind _movementdir (Variables|Default|GetMovementDir))
  (bind (_x _y _z) (Math|Vector|BreakVector _movementdir))
  (|CallParentFunction DeltaSeconds)
  (Variables|Default|SetAlphaValue (+ (Variables|Default|GetAlphaValue) (* DeltaSeconds (Variables|Default|GetAlphaScale))))
  (Transformation|SetActorLocation (+ (Variables|Default|GetDefaultLocation) (Math|Vector|MakeVector (* _x (Math|Float|Lerp 0.0 3e+02 (Math|Float|Absolute(Float) (- (Math|Float|%(Float) (Variables|Default|GetAlphaValue) 2.0) 1.0)))) (* _y (Math|Float|Lerp 0.0 3e+02 (Math|Float|Absolute(Float) (- (Math|Float|%(Float) (Variables|Default|GetAlphaValue) 2.0) 1.0)))) (* _z (Math|Float|Lerp 0.0 3e+02 (Math|Float|Absolute(Float) (- (Math|Float|%(Float) (Variables|Default|GetAlphaValue) 2.0) 1.0)))))) false false))

(fn ConstructionScript
  (|CallParentFunction))

(fn MergeBlock
  (params (BlockType :type BlockType%20Enum :default "NewEnumerator0"))
  (|CallParentFunction BlockType)
  (Utilities|FlowControl|Sequence
    (:then_0
      (if (Utilities|Enum|Equal(Enum) BlockType "NewEnumerator7")
        (Rendering|SetVisibility (Variables|Default|GetWidget) true false)
        (Variables|Default|SetIs%20Time true)))
    (:then_1
      (if (and (Utilities|Enum|Equal(Enum) BlockType "NewEnumerator1") (Variables|Default|GetIs%20Time))
        (Rendering|SetVisibility (Variables|Default|GetWidget) false false)
        (Variables|Default|SetAlphaScale 0.5)
        (Components|DestroyComponent (Variables|Default|GetCollision))))))