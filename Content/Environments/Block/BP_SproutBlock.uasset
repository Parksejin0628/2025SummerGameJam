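; BP_SproutBlock is a block that grows a line of tree blocks in response to merges with other blocks.
; Its MergeBlock override calls the parent; one block type arms it by setting IsTime, showing its widget and playing a pickup sound.
; While armed, a second type hides the widget and spawns three BP_TreeBlocks spaced along GrowDir, each with a success sound.
; IsTime is never cleared here.
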(event EventBeginPlay
  (|CallParentFunction))

(event Collision|EventActorBeginOverlap
  (params (OtherActor :type Actor%20Object%20Reference))
  (|CallParentFunction OtherActor) ; This node is disabled and will not be called.\nDrag off pins to build functionality.
)

(event EventTick
  (params (DeltaSeconds :type Float%20%28single-precision%29))
  (|CallParentFunction DeltaSeconds) ; This node is disabled and will not be called.\nDrag off pins to build functionality.
)

(fn ConstructionScript
  (|CallParentFunction))

(fn MergeBlock
  (params (BlockType :type BlockType%20Enum :default "NewEnumerator0"))
  (bind _returnvalue (Transformation|GetActorTransform))
  (bind (_location _rotation _scale) (Math|Transform|BreakTransform _returnvalue))
  (|CallParentFunction BlockType)
  (Utilities|FlowControl|Sequence
    (:then_0
      (if (Utilities|Enum|Equal(Enum) BlockType "NewEnumerator7")
        (Rendering|SetVisibility (Variables|Default|GetWidget) true false)
        (Variables|Default|SetbIsTime true)
        (bind _asbp_game_instance (Utilities|Casting|CastToBP_GameInstance (Game|GetGameInstance)))
        (Default|PlaySound _asbp_game_instance "/Game/Sound/SFx/큐브_획득.큐브_획득")))
    (:then_1
      (if (and (Utilities|Enum|Equal(Enum) BlockType "NewEnumerator0") (Variables|Default|GetbIsTime))
        (Rendering|SetVisibility (Variables|Default|GetWidget) false false)
        (for _index (range 1 3)
          (Game|SpawnActorfromClass "/Game/Environments/Block/BP_TreeBlock.BP_TreeBlock_C" (Math|Transform|MakeTransform (+ (Transformation|GetActorLocation) (* (Variables|Default|GetGrowDir) (* 1e+02 _index))) _rotation _scale) "Undefined" "MultiplyWithRoot" 0 0)
          (bind _asbp_game_instance_2 (Utilities|Casting|CastToBP_GameInstance (Game|GetGameInstance)))
          (Default|PlaySound _asbp_game_instance_2 "/Game/Sound/SFx/블록_상호작용_성공.블록_상호작용_성공"))))))