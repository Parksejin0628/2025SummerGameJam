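; BP_AirBlock is an invisible-style block variant that can turn into a normal block through merging.
; On BeginPlay it runs the parent logic, then applies a transparent material to its BodyBox.
; Its MergeBlock override calls the parent, then for one specific block type spawns BP_Normal at its own transform and destroys itself.
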(event EventBeginPlay
  (|CallParentFunction)
  (Rendering|Material|SetMaterial (Variables|Default|GetBodyBox) 0 "/Game/Assets/Aura/M_Transparent.M_Transparent"))

(event Collision|EventActorBeginOverlap
  (params (OtherActor :type Actor%20Object%20Reference))
  (|CallParentFunction OtherActor) ; This node is disabled and will not be called.\nDrag off pins to build functionality.
)

(event EventTick
  (params (DeltaSeconds :type Float%20%28single-precision%29))
  (|CallParentFunction DeltaSeconds) ; This node is disabled and will not be called.\nDrag off pins to build functionality.
)

(fn ConstructionScript
  (|CallParentFunction))

(fn MergeBlock
  (params (BlockType :type BlockType%20Enum :default "NewEnumerator0"))
  (|CallParentFunction BlockType)
  (if (Utilities|Enum|Equal(Enum) BlockType "NewEnumerator5")
    (Game|SpawnActorfromClass "/Game/Environments/Block/BP_Normal.BP_Normal_C" (Transformation|GetActorTransform) "Undefined" "MultiplyWithRoot" 0 0)
    (Actor|DestroyActor)))