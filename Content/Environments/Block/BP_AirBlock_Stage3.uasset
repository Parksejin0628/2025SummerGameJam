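; BP_AirBlock_Stage3 is an air block variant, derived from a parent block class, that turns into another block when merged.
; On BeginPlay it makes its body box transparent.
; Its MergeBlock override calls the parent, then checks the incoming block type and spawns either a BP_Normal or a BP_HotAir at its own transform.
; On a match it also plays the interaction success sound through BP_GameInstance and destroys itself.
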(event EventBeginPlay
  (|CallParentFunction)
  (Rendering|Material|SetMaterial (Variables|Default|GetBodyBox) 0 "/Game/Assets/Aura/M_Transparent.M_Transparent"))

(event Collision|EventActorBeginOverlap
  (params (OtherActor :type Actor%20Object%20Reference))
  (|CallParentFunction OtherActor) ; This node is disabled and will not be called.\nDrag off pins to build functionality.
)

(event EventTick
  (params (DeltaSeconds :type Float%20%28single-precision%29))
  (|CallParentFunction DeltaSeconds) ; This node is disabled and will not be called.\nDrag off pins to build functionality.
)

(fn ConstructionScript
  (|CallParentFunction))

(fn MergeBlock
  (params (BlockType :type BlockType%20Enum :default "NewEnumerator0"))
  (|CallParentFunction BlockType)
  (Utilities|FlowControl|Sequence
    (:then_0
      (if (Utilities|Enum|Equal(Enum) BlockType "NewEnumerator5")
        (Game|SpawnActorfromClass "/Game/Environments/Block/BP_Normal.BP_Normal_C" (Transformation|GetActorTransform) "Undefined" "MultiplyWithRoot" 0 0)
        (bind _asbp_game_instance (Utilities|Casting|CastToBP_GameInstance (Game|GetGameInstance)))
        (Default|PlaySound _asbp_game_instance "/Game/Sound/SFx/블록_상호작용_성공.블록_상호작용_성공")
        (Actor|DestroyActor)))
    (:then_1
      (if (Utilities|Enum|Equal(Enum) BlockType "NewEnumerator0")
        (Game|SpawnActorfromClass "/Game/Environments/Block/BP_HotAir.BP_HotAir_C" (Transformation|GetActorTransform) "Undefined" "MultiplyWithRoot" 0 0)
        (bind _asbp_game_instance_2 (Utilities|Casting|CastToBP_GameInstance (Game|GetGameInstance)))
        (Default|PlaySound _asbp_game_instance_2 "/Game/Sound/SFx/블록_상호작용_성공.블록_상호작용_성공")
        (Actor|DestroyActor)))))