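; BP_HotAir is an invisible hot-air block that becomes an updraft and launches the player upward.
; BeginPlay makes its body box transparent, and MergeBlock with one specific block type enables the updraft, shows its effect and plays a success sound through the game instance.
; While active, overlap by a Player-tagged BP_Stage3_Player triggers LaunchCharacter, adding upward velocity to existing motion rather than overriding it.
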(event EventBeginPlay
  (|CallParentFunction)
  (Rendering|Material|SetMaterial (Variables|Default|GetBodyBox) 0 "/Game/Assets/Aura/M_Transparent.M_Transparent"))

(event Collision|EventActorBeginOverlap
  (params (OtherActor :type Actor%20Object%20Reference))
  (|CallParentFunction OtherActor)
  (if (Variables|Default|GetbIsUpdraft)
    (if (Actor|ActorHasTag OtherActor "Player")
      (Development|PrintString "Jump Up!")
      (bind _asbp_stage_3_player (Utilities|Casting|CastToBP_Stage3_Player OtherActor))
      (Character|LaunchCharacter _asbp_stage_3_player "0.000000,0.000000,1300.000000" false false))))

(event EventTick
  (params (DeltaSeconds :type Float%20%28single-precision%29))
  (|CallParentFunction DeltaSeconds) ; This node is disabled and will not be called.\nDrag off pins to build functionality.
)

(fn ConstructionScript
  (|CallParentFunction))

(fn MergeBlock
  (params (BlockType :type BlockType%20Enum :default "NewEnumerator0"))
  (|CallParentFunction BlockType)
  (if (Utilities|Enum|Equal(Enum) BlockType "NewEnumerator3")
    (Variables|Default|SetbIsUpdraft true)
    (Rendering|SetVisibility (Variables|Default|GetUpdraftFx) true false)
    (bind _asbp_game_instance (Utilities|Casting|CastToBP_GameInstance (Game|GetGameInstance)))
    (Default|PlaySound _asbp_game_instance "/Game/Sound/SFx/블록_상호작용_성공.블록_상호작용_성공")))