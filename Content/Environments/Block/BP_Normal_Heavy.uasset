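; BP_Normal_Heavy is a heavy block variant that destroys tree blocks beneath it and moves when unobstructed.
; Each tick, a short downward line trace destroys any BP_TreeBlock it hits, then the block offsets itself locally by Delta scaled by frame time unless IsOverlap is set.
; Overlap begin and end events toggle that flag, ignoring BP_AirBlock_Stage3, while construction and MergeBlock defer to the parent.
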(event EventBeginPlay
  (|CallParentFunction))

(event Collision|EventActorBeginOverlap
  (params (OtherActor :type Actor%20Object%20Reference))
  (|CallParentFunction OtherActor)
  (Utilities|Casting|CastToBP_AirBlock_Stage3 OtherActor
    (:CastFailed
      (Variables|Default|SetbIsOverlap true))))

(event EventTick
  (params (DeltaSeconds :type Float%20%28single-precision%29))
  (|CallParentFunction DeltaSeconds)
  (Utilities|FlowControl|Sequence
    (:then_0
      (bind _outhit (Collision|LineTraceByChannel (Transformation|GetActorLocation) (+ (Transformation|GetActorLocation) "0.000000,0.000000,-60.000000") "TraceTypeQuery3" false 0 "None"))
      (bind _asbp_tree_block (Utilities|Casting|CastToBP_TreeBlock (.HitActor (Collision|BreakHitResult _outhit))))
      (Actor|DestroyActor _asbp_tree_block))
    (:then_1
      (if (not (Variables|Default|GetbIsOverlap))
        (Transformation|AddActorLocalOffset (* (Variables|Default|GetDelta) DeltaSeconds) false false)))))

(event Collision|EventActorEndOverlap
  (params (OtherActor :type Actor%20Object%20Reference))
  (Utilities|Casting|CastToBP_AirBlock_Stage3 OtherActor
    (:CastFailed
      (Variables|Default|SetbIsOverlap false))))

(fn ConstructionScript
  (|CallParentFunction))

(fn MergeBlock
  (params (BlockType :type BlockType%20Enum :default "NewEnumerator0"))
  (|CallParentFunction BlockType))