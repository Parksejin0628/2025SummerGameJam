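; BP_WaterBlock is an environment water block that can turn into an ice block when merged.
; It overrides MergeBlock, calls the parent logic, then checks the incoming block type against one enum value.
; On a match it spawns BP_IceBlock at its own transform and destroys itself.
; BeginPlay and the construction script only call their parents, and Tick and overlap are disabled.
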(event EventBeginPlay
  (|CallParentFunction))

(event Collision|EventActorBeginOverlap
  (params (OtherActor :type Actor%20Object%20Reference))
  (|CallParentFunction OtherActor) ; This node is disabled and will not be called.\nDrag off pins to build functionality.
)

(event EventTick
  (params (DeltaSeconds :type Float%20%28single-precision%29))
  (|CallParentFunction DeltaSeconds) ; This node is disabled and will not be called.\nDrag off pins to build functionality.
)

(fn ConstructionScript
  (|CallParentFunction))

(fn MergeBlock
  (params (BlockType :type BlockType%20Enum :default "NewEnumerator0"))
  (|CallParentFunction BlockType)
  (Utilities|FlowControl|Sequence
    (:then_0
      (if (Utilities|Enum|Equal(Enum) BlockType "NewEnumerator1")
        (Game|SpawnActorfromClass "/Game/Environments/Block/BP_IceBlock.BP_IceBlock_C" (Transformation|GetActorTransform) "Undefined" "MultiplyWithRoot" 0 0)
        (Actor|DestroyActor)))))