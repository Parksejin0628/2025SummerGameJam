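; BP_Tesseract is a Tesseract pickup that sends the player on to another level.
; Tick spins it on all three axes and slowly scales it up once triggered.
; Overlap with a Player-tagged actor triggers it, shows a white fade-out widget and plays the acquisition sound through BP_GameInstance.
; It also stores LevelName as the game instance's next map, then opens the Loading level after a delay.
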(event EventBeginPlay)

(event Collision|EventActorBeginOverlap
  (params (OtherActor :type Actor%20Object%20Reference))
  (Development|PrintString "Overlap")
  (if (Actor|ActorHasTag OtherActor "Player")
    (Variables|Default|SetbIsTrigger true)
    (bind _returnvalue (UserInterface|CreateWidget "/Game/UI/WBP_PadeOut_White.WBP_PadeOut_White_C"))
    (UserInterface|Viewport|AddtoViewport _returnvalue 0)
    (bind _asbp_game_instance (Utilities|Casting|CastToBP_GameInstance (Game|GetGameInstance)))
    (Default|PlaySound _asbp_game_instance "/Game/Sound/SFx/테서랙트_획득.테서랙트_획득")
    (Variables|/Game/Core/BP_GameInstance.BP_GameInstance_C|SetNextLoadingMap _asbp_game_instance (Variables|Default|GetLevelName))
    (Utilities|FlowControl|Delay 5.0)
    (Game|OpenLevel(byName) "Loading")))

(event EventTick
  (params (DeltaSeconds :type Float%20%28single-precision%29))
  (bind _returnvalue (Transformation|GetActorRotation))
  (bind (_roll _pitch _yaw) (Math|Rotator|BreakRotator _returnvalue))
  (Utilities|FlowControl|Sequence
    (:then_0
      (Transformation|SetActorRotation (Math|Rotator|MakeRotator (+ (* DeltaSeconds 1e+01) _roll) (+ (* DeltaSeconds 5e+01) _pitch) (+ (* DeltaSeconds 3e+01) _yaw))))
    (:then_1
      (if (Variables|Default|GetbIsTrigger)
        (Transformation|SetActorScale3D (+ (Transformation|GetActorScale3D) (* DeltaSeconds "0.010000,0.010000,0.010000")))))))

(fn ConstructionScript)