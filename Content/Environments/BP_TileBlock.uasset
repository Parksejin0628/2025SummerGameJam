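; BP_TileBlock is a tile actor that can be highlighted and merged with a block type.
; OnBlockClicked shows or hides OutLineBox, and BeginPlay sets a custom depth stencil value on BodyBox.
; MergeBlock prints the type, hides the outline, then spawns the matching colored cube Blueprint at the tile's transform through per-type branches.
; The tile is not destroyed afterward, and one enumerator value has no branch.
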(event Custom|OnBlockClicked
  (params (bIsActivate :type Boolean))
  (Rendering|SetVisibility (Variables|Default|GetOutLineBox) bIsActivate false))

(event EventBeginPlay
  (Rendering|SetCustomDepthStencilValue (Variables|Default|GetBodyBox) 1))

(event Collision|EventActorBeginOverlap
  (params (OtherActor :type Actor%20Object%20Reference)))

(event EventTick
  (params (DeltaSeconds :type Float%20%28single-precision%29)))

(fn ConstructionScript)

(fn MergeBlock
  (params (BlockType :type BlockType%20Enum :default "NewEnumerator0"))
  (Development|PrintString (Utilities|String|Append "Merge block with" (Utilities|String|EnumtoString BlockType)))
  (Rendering|SetVisibility (Variables|Default|GetOutLineBox) false false)
  (Utilities|FlowControl|Sequence
    (:then_0
      (if (Utilities|Enum|Equal(Enum) BlockType "NewEnumerator0")
        (Game|SpawnActorfromClass "/Game/Environments/Cube/BP_Cube_Red.BP_Cube_Red_C" (Transformation|GetActorTransform) "Undefined" "MultiplyWithRoot" 0 0)))
    (:then_1
      (if (Utilities|Enum|Equal(Enum) BlockType "NewEnumerator1")
        (Game|SpawnActorfromClass "/Game/Environments/Cube/BP_Cube_Blue.BP_Cube_Blue_C" (Transformation|GetActorTransform) "Undefined" "MultiplyWithRoot" 0 0)))
    (:then_2
      (if (Utilities|Enum|Equal(Enum) BlockType "NewEnumerator2")
        (Game|SpawnActorfromClass "/Game/Environments/Cube/BP_Cube_Ornage.BP_Cube_Ornage_C" (Transformation|GetActorTransform) "Undefined" "MultiplyWithRoot" 0 0)))
    (:then_3
      (if (Utilities|Enum|Equal(Enum) BlockType "NewEnumerator3")
        (Game|SpawnActorfromClass "/Game/Environments/Cube/BP_Cube_White.BP_Cube_White_C" (Transformation|GetActorTransform) "Undefined" "MultiplyWithRoot" 0 0)))
    (:then_4
      (if (Utilities|Enum|Equal(Enum) BlockType "NewEnumerator5")
        (Game|SpawnActorfromClass "/Game/Environments/Cube/BP_Cube_Gray.BP_Cube_Gray_C" (Transformation|GetActorTransform) "Undefined" "MultiplyWithRoot" 0 0)))
    (:then_5
      (if (Utilities|Enum|Equal(Enum) BlockType "NewEnumerator6")
        (Game|SpawnActorfromClass "/Game/Environments/Cube/BP_Cube_Black.BP_Cube_Black_C" (Transformation|GetActorTransform) "Undefined" "MultiplyWithRoot" 0 0)))
    (:then_6
      (if (Utilities|Enum|Equal(Enum) BlockType "NewEnumerator7")
        (Game|SpawnActorfromClass "/Game/Environments/Cube/BP_Cube_Gold.BP_Cube_Gold_C" (Transformation|GetActorTransform) "Undefined" "MultiplyWithRoot" 0 0)))))